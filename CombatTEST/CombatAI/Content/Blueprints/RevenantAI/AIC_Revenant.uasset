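; AI controller for the Revenant enemy that runs its behavior tree and handles player sighting and facing.
; On BeginPlay it starts BT_Revenant and caches its BP_Revenant through the instigator.
; Pawn sensing raises the "SeePlayer?" blackboard flag, and a retriggerable delay clears it five seconds after the last sighting.
; Tick smoothly lerps the Revenant's yaw toward the blackboard's MoveToNewDestination vector.
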(event `self.ReceiveTick`
  (params (DeltaSeconds :type "Float (single-precision)"))
  (bind _revenant_enemy (`self.Revenant Enemy`))
  (bind (_returnvalue_roll _returnvalue_pitch _returnvalue_yaw) (`KismetMathLibrary.BreakRotator` (`KismetMathLibrary.RLerp` (`self.K2_GetActorRotation` _revenant_enemy) (`KismetMathLibrary.FindLookAtRotation` (`self.K2_GetActorLocation` _revenant_enemy) (`BlackboardComponent.GetValueAsVector` (`AIBlueprintHelperLibrary.GetBlackboard` null) "MoveToNewDestination")) 0.025 true)))
  ;[0 1 0.6842] Turn To Target
  (`self.K2_SetActorRotation` _revenant_enemy (`KismetMathLibrary.MakeRotator` 0.0 0.0 _returnvalue_yaw) false))

(event `self.ReceiveBeginPlay`
  ;[0 0 0] Initialize Revenant AI
  (`self.RunBehaviorTree` "/Game/Blueprints/RevenantAI/BT_Revenant.BT_Revenant")
  (bind _asbp_revenant (cast `/Game/Blueprints/BP_Revenant` (`self.GetInstigator`)))
  (set `self.Revenant Enemy` _asbp_revenant))

(event `self.PawnSensing.OnSeePawn`
  (params (Pawn :type "Pawn Object Reference"))
  ;[1 0 0] If Player is Seen, Chase
  (`|ExecutionSequence`
    (:`then_0`
      (`BlackboardComponent.SetValueAsBool` (`AIBlueprintHelperLibrary.GetBlackboard` null) "SeePlayer?" true))
    (:`then_1`
      (`KismetSystemLibrary.RetriggerableDelay` 5.0)
      (`BlackboardComponent.SetValueAsBool` (`AIBlueprintHelperLibrary.GetBlackboard` null) "SeePlayer?" false))))

(fn `UserConstructionScript`)