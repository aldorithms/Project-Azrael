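; BP_Revenant is an enemy character with per-limb hitboxes that loses health and stagger when struck by first-person projectiles.
; Head hits set a critical flag, which Stagger clears before Damage reads it; UpperLegL hits trigger neither function.
; Depleted stagger plays a random hit montage and refills, while zero health ragdolls the mesh with an impulse.
; Any damage sets the blackboard's "SeePlayer?" key to true.
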(event `self.ReceiveBeginPlay`
  (set `self.CurrentStagger` 100.0)
  (set `self.Current Health` 1000.0))

(event `self.TorsoHitbox.OnComponentHit`
  (params (HitComponent :type "PrimitiveComponent Object Reference") (OtherActor :type "Actor Object Reference") (OtherComp :type "PrimitiveComponent Object Reference") (NormalImpulse :type "Vector Structure") (Hit :type "HitResult Structure (by ref)"))
  ;[0 0 1] Non-Critical Hit
  (set `self.Hit` Hit)
  (cast `/Game/FirstPerson/Blueprints/BP_FirstPersonProjectile` OtherActor)
  (`self.Stagger` :!label _label)
  (`self.Damage`))

(event `self.HeadHitbox.OnComponentHit`
  (params (HitComponent :type "PrimitiveComponent Object Reference") (OtherActor :type "Actor Object Reference") (OtherComp :type "PrimitiveComponent Object Reference") (NormalImpulse :type "Vector Structure") (Hit :type "HitResult Structure (by ref)"))
  ;[1 0 0] Critical Hit
  (set `self.Hit` Hit)
  (cast `/Game/FirstPerson/Blueprints/BP_FirstPersonProjectile` OtherActor)
  (set `self.IsCritical?` true)
  (`self.Stagger`)
  (`self.Damage`))

(event `self.LowerLegL.OnComponentHit`
  (params (HitComponent :type "PrimitiveComponent Object Reference") (OtherActor :type "Actor Object Reference") (OtherComp :type "PrimitiveComponent Object Reference") (NormalImpulse :type "Vector Structure") (Hit :type "HitResult Structure (by ref)"))
  ;[0 0 1] Non-Critical Hit
  (set `self.Hit` Hit)
  (cast `/Game/FirstPerson/Blueprints/BP_FirstPersonProjectile` OtherActor)
  (goto _label))

(event `self.ReceiveAnyDamage`
  (params (Damage :type "Float (single-precision)") (DamageType :type "DamageType Object Reference") (InstigatedBy :type "Controller Object Reference") (DamageCauser :type "Actor Object Reference"))
  ;[0 1 0.717] Hit Reaction
  (`BlackboardComponent.SetValueAsBool` (`AIBlueprintHelperLibrary.GetBlackboard` null) "SeePlayer?" true))

(event `self.LowerLegR.OnComponentHit`
  (params (HitComponent :type "PrimitiveComponent Object Reference") (OtherActor :type "Actor Object Reference") (OtherComp :type "PrimitiveComponent Object Reference") (NormalImpulse :type "Vector Structure") (Hit :type "HitResult Structure (by ref)"))
  ;[0 0 1] Non-Critical Hit
  (set `self.Hit` Hit)
  (cast `/Game/FirstPerson/Blueprints/BP_FirstPersonProjectile` OtherActor)
  (goto _label))

(event `self.UpperLegL.OnComponentHit`
  (params (HitComponent :type "PrimitiveComponent Object Reference") (OtherActor :type "Actor Object Reference") (OtherComp :type "PrimitiveComponent Object Reference") (NormalImpulse :type "Vector Structure") (Hit :type "HitResult Structure (by ref)"))
  ;[0 0 1] Non-Critical Hit
  (set `self.Hit` Hit)
  (cast `/Game/FirstPerson/Blueprints/BP_FirstPersonProjectile` OtherActor))

(event `self.UpperLegR.OnComponentHit`
  (params (HitComponent :type "PrimitiveComponent Object Reference") (OtherActor :type "Actor Object Reference") (OtherComp :type "PrimitiveComponent Object Reference") (NormalImpulse :type "Vector Structure") (Hit :type "HitResult Structure (by ref)"))
  ;[0 0 1] Non-Critical Hit
  (set `self.Hit` Hit)
  (cast `/Game/FirstPerson/Blueprints/BP_FirstPersonProjectile` OtherActor)
  (goto _label))

(event `self.HandL.OnComponentHit`
  (params (HitComponent :type "PrimitiveComponent Object Reference") (OtherActor :type "Actor Object Reference") (OtherComp :type "PrimitiveComponent Object Reference") (NormalImpulse :type "Vector Structure") (Hit :type "HitResult Structure (by ref)"))
  ;[0 0 1] Non-Critical Hit
  (set `self.Hit` Hit)
  (cast `/Game/FirstPerson/Blueprints/BP_FirstPersonProjectile` OtherActor)
  (goto _label))

(event `self.HandR.OnComponentHit`
  (params (HitComponent :type "PrimitiveComponent Object Reference") (OtherActor :type "Actor Object Reference") (OtherComp :type "PrimitiveComponent Object Reference") (NormalImpulse :type "Vector Structure") (Hit :type "HitResult Structure (by ref)"))
  ;[0 0 1] Non-Critical Hit
  (set `self.Hit` Hit)
  (cast `/Game/FirstPerson/Blueprints/BP_FirstPersonProjectile` OtherActor)
  (goto _label))

(event `self.LowerArmL.OnComponentHit`
  (params (HitComponent :type "PrimitiveComponent Object Reference") (OtherActor :type "Actor Object Reference") (OtherComp :type "PrimitiveComponent Object Reference") (NormalImpulse :type "Vector Structure") (Hit :type "HitResult Structure (by ref)"))
  ;[0 0 1] Non-Critical Hit
  (set `self.Hit` Hit)
  (cast `/Game/FirstPerson/Blueprints/BP_FirstPersonProjectile` OtherActor)
  (goto _label))

(event `self.LowerArmR.OnComponentHit`
  (params (HitComponent :type "PrimitiveComponent Object Reference") (OtherActor :type "Actor Object Reference") (OtherComp :type "PrimitiveComponent Object Reference") (NormalImpulse :type "Vector Structure") (Hit :type "HitResult Structure (by ref)"))
  ;[0 0 1] Non-Critical Hit
  (set `self.Hit` Hit)
  (cast `/Game/FirstPerson/Blueprints/BP_FirstPersonProjectile` OtherActor)
  (goto _label))

(event `self.UpperArmL.OnComponentHit`
  (params (HitComponent :type "PrimitiveComponent Object Reference") (OtherActor :type "Actor Object Reference") (OtherComp :type "PrimitiveComponent Object Reference") (NormalImpulse :type "Vector Structure") (Hit :type "HitResult Structure (by ref)"))
  ;[0 0 1] Non-Critical Hit
  (set `self.Hit` Hit)
  (cast `/Game/FirstPerson/Blueprints/BP_FirstPersonProjectile` OtherActor)
  (goto _label))

(event `self.UpperArmR.OnComponentHit`
  (params (HitComponent :type "PrimitiveComponent Object Reference") (OtherActor :type "Actor Object Reference") (OtherComp :type "PrimitiveComponent Object Reference") (NormalImpulse :type "Vector Structure") (Hit :type "HitResult Structure (by ref)"))
  ;[0 0 1] Non-Critical Hit
  (set `self.Hit` Hit)
  (cast `/Game/FirstPerson/Blueprints/BP_FirstPersonProjectile` OtherActor)
  (goto _label))

(fn `Damage`
  (if (`self.IsCritical?`)
    (set `self.IsCritical?` false)
    (`KismetSystemLibrary.LogString` "Head Shot!")
    (bind _returnvalue (`GameplayStatics.ApplyDamage` self (`self.CritDamage`) null (`self.Projectile`)))
    (set `self.Current Health` (`KismetMathLibrary.FClamp` (- (`self.Current Health`) _returnvalue) 0.0 (`self.MaxHealth`)))
    (else
      (`KismetSystemLibrary.LogString` "Body Shot!")
      (bind _returnvalue_2 (`GameplayStatics.ApplyDamage` self (`self.BaseDamage`) null (`self.Projectile`)))
      (set `self.Current Health` (`KismetMathLibrary.FClamp` (- (`self.Current Health`) _returnvalue_2) 0.0 (`self.MaxHealth`)))))
  ;[0 0 0] Check If Dead
  (if (== (`self.Current Health`) 0.0)
    (`self.Death`)
    (else
      (return))))

(fn `Death`
  (bind _mesh (`self.Mesh`))
  (`PrimitiveComponent.SetCollisionEnabled` (`self.CapsuleComponent`) "NoCollision")
  (`PrimitiveComponent.SetSimulatePhysics` _mesh true)
  (`PrimitiveComponent.SetCollisionEnabled` _mesh "PhysicsOnly")
  (`PrimitiveComponent.AddImpulse` _mesh (* (`.ImpactNormal` (`GameplayStatics.BreakHitResult` (`self.Hit`))) 1500.0) "None" true))

(fn `Stagger`
  (if (`self.IsCritical?`)
    (set `self.IsCritical?` false)
    (`KismetSystemLibrary.LogString` "Head Shot!")
    (bind _returnvalue (`GameplayStatics.ApplyDamage` self (`self.CritStaggerDamage`) null (`self.Projectile`)))
    (set `self.CurrentStagger` (`KismetMathLibrary.FClamp` (- (`self.CurrentStagger`) _returnvalue) 0.0 (`self.MaxStagger`)))
    (else
      (`KismetSystemLibrary.LogString` "Body Shot!")
      (bind _returnvalue_2 (`GameplayStatics.ApplyDamage` self (`self.BaseStaggerDamage`) null (`self.Projectile`)))
      (set `self.CurrentStagger` (`KismetMathLibrary.FClamp` (- (`self.CurrentStagger`) _returnvalue_2) 0.0 (`self.MaxStagger`)))))
  ;[0 0 0] Check If Staggered
  (if (== (`self.CurrentStagger`) 0.0)
    (`self.PlayAnimMontage` (`|GetArrayItem` (`self.getBaseHitAnimations`) (`KismetMathLibrary.RandomIntegerInRange` 0 (`KismetArrayLibrary.Array_Length` (`self.getBaseHitAnimations`)))) 0.75)
    (set `self.CurrentStagger` (`self.MaxStagger`))
    (return)
    (else
      (return))))

(fn `UserConstructionScript`)